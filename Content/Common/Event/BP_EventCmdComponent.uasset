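; Actor component that runs data-table-driven scripted events as a sequence of command objects.
; Start builds a command object per EventDataTable row via class-mapping tables, begins at a label, and EndEventCmd advances, jumps or finishes; Cancel aborts.
; Registerable DataTable lists resolve names to command classes, sounds, level sequences, montages and widgets.
; It also keeps a named flag set and controls 2D sound and sequence playback.
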(event `self.ReceiveBeginPlay`
  (set `self.PlayerController` (`GameplayStatics.GetPlayerController` 0)))

(fn `AddEventCmdClassMapping`
  (params (InDataTable :type "CompositeDataTable Object Reference"))
  (`KismetArrayLibrary.Array_Add` (`self.EventCmdClassMapping`) InDataTable))

(fn `AddEventMontageMapping`
  (params (InDataTable :type "CompositeDataTable Object Reference"))
  (`KismetArrayLibrary.Array_Add` (`self.EventMontageMapping`) InDataTable))

(fn `AddEventSequenceMapping`
  (params (InDataTable :type "CompositeDataTable Object Reference"))
  (`KismetArrayLibrary.Array_Add` (`self.EventSequenceMapping`) InDataTable))

(fn `AddEventSoundMapping`
  (params (InDataTable :type "CompositeDataTable Object Reference"))
  (`KismetArrayLibrary.Array_Add` (`self.EventSoundMapping`) InDataTable))

(fn `AddEventWidgetMapping`
  (params (InDataTable :type "CompositeDataTable Object Reference"))
  (`KismetArrayLibrary.Array_Add` (`self.EventWidgetMapping`) InDataTable))

(fn `Cancel`
  (`/Engine/EditorBlueprintResources/StandardMacros.IsValid` (`self.GetCrtEventCmd`)
    (:`Is Valid`
      (`/Game/Common/Event/EventCmds/BPEC_Base.OnEnd` (`self.GetCrtEventCmd`) true)
      (set `self.CrtIndex` -1))
    (:`Is Not Valid`
      _))
  (set `self.CrtIndex` -1)
  (`self.OnEnd`))

(fn `CreateEventCmd`
  (params (InLabel :type "Name (by ref)") (InCommand :type "Name (by ref)") (InArgs :type "Array of String (by ref)"))
  (returns (OutEventCmd :type "/Game/Common/Event/EventCmds/BPEC_Base Object Reference"))
  (locals (EventCmdClass :type "/Game/Common/Event/EventCmds/BPEC_Base Class Reference"))
  (bind _output_get (set `local.EventCmdClass` (`self.FindEventCmdClass` (`local.InCommand`))))
  (if (`KismetSystemLibrary.IsValidClass` _output_get)
    (bind _returnvalue (`|GenericCreateObject` (`local.EventCmdClass`) self self (`local.InLabel`) (`local.InArgs`)))
    (return _returnvalue)
    (else
      (return null))))

(fn `CreateEventCmds`
  (params (InDataTable :type "DataTable Object Reference"))
  (locals (DataTable :type "DataTable Object Reference") (Label :type Name) (EventCmd :type "/Game/Common/Event/EventCmds/BPEC_Base Object Reference") (CommandName :type Name :default "None"))
  (`KismetArrayLibrary.Array_Clear` (`self.EventCmds`))
  (bind _outrownames (`DataTableFunctionLibrary.GetDataTableRowNames` (`local.InDataTable`)))
  (for _array_element _outrownames
    (set `local.Label` _array_element)
    (bind _returnvalue (`|GetDataTableRow` (`local.InDataTable`) (`local.Label`))
      (:`then`
        (bind (_command _args) (break `/Game/Common/Event/FEventCmd` _returnvalue))
        (set `local.CommandName` _command)
        (bind _outeventcmd (`self.CreateEventCmd` (`local.Label`) (`local.CommandName`) _args))
        (bind _output_get (set `local.EventCmd` _outeventcmd))
        (`/Engine/EditorBlueprintResources/StandardMacros.IsValid` _output_get
          (:`Is Valid`
            (`KismetArrayLibrary.Array_Add` (`self.EventCmds`) (`local.EventCmd`)))
          (:`Is Not Valid`
            (`KismetSystemLibrary.PrintString` (`KismetStringLibrary.Concat_StrStr` "CreateEventCmd not found command : " (`KismetStringLibrary.Conv_NameToString` (`local.CommandName`))) true true (struct :`R` 1.0 :`B` 1.0 :`A` 1.0))))))))

(fn `CreateEventWidget`
  (params (InWidgetClass :type "/Game/Common/Event/Widgets/WBP_EventWidget Class Reference") (EventCmd :type "/Game/Common/Event/EventCmds/BPEC_Base Object Reference") (Args :type "Array of String"))
  (returns (ReturnValue :type "UserWidget Object Reference"))
  (bind _returnvalue (`|CreateWidget` InWidgetClass null EventCmd Args))
  (return _returnvalue))

(fn `EndEventCmd`
  (params (InNextIndex :type Integer :default -1) (InEnd :type Boolean))
  (`/Game/Common/Event/EventCmds/BPEC_Base.OnEnd` (`self.GetCrtEventCmd`) false)
  (set `self.CrtIndex` (`KismetMathLibrary.SelectInt` (`local.InNextIndex`) (+ (`self.CrtIndex`) 1) (>= (`local.InNextIndex`) 0)))
  (if (or (`local.InEnd`) (not (`KismetArrayLibrary.Array_IsValidIndex` (`self.EventCmds`) (`self.CrtIndex`))))
    (set `self.CrtIndex` -1)
    (`self.OnEnd`)
    (`KismetArrayLibrary.Array_Clear` (`self.EventCmds`))
    (else
      (`self.Exec`))))

(fn `Exec`
  (`/Game/Common/Event/EventCmds/BPEC_Base.OnStarted` (`self.GetCrtEventCmd`)))

(fn `FindEventCmdClass`
  (params (InCommand :type Name))
  (returns (EventCmdClass :type "/Game/Common/Event/EventCmds/BPEC_Base Class Reference") (IsFound :type Boolean))
  (for _array_element (`self.EventCmdClassMapping`)
    (bind _returnvalue (`|GetDataTableRow` _array_element (`local.InCommand`))
      (:`then`
        (return (`.EventCmdClass_2_A3B73D224EB74E0202933CBB35B6E459` (break `/Game/Common/Event/FEventCmdClass` _returnvalue)) true))))
  (return null false))

(fn `FindEventMontage`
  (params (InName :type Name))
  (returns (Montage :type "AnimMontage Object Reference"))
  (locals (Name :type String) (Seq :type "LevelSequenceActor Object Reference"))
  (for _array_element (`self.EventMontageMapping`)
    (bind _returnvalue (`|GetDataTableRow` _array_element (`local.InName`))
      (:`then`
        (return (`.Montage_6_D05F76FC47EBEDEC836A18B2123F30B4` (break `/Game/Common/Event/FEventMontage` _returnvalue))))))
  (return null))

(fn `FindEventSound`
  (params (InCommand :type Name))
  (returns (EventCmdClass :type "SoundBase Object Reference") (IsFound :type Boolean))
  (for _array_element (`self.EventSoundMapping`)
    (bind _returnvalue (`|GetDataTableRow` _array_element (`local.InCommand`))
      (:`then`
        (return (`.Sound_4_D05F76FC47EBEDEC836A18B2123F30B4` (break `/Game/Common/Event/FEventSound` _returnvalue)) true))))
  (return null false))

(fn `FindEventWidget`
  (params (InName :type Name))
  (returns (Widget :type "/Game/Common/Event/Widgets/WBP_EventWidget Class Reference"))
  (locals (Name :type String) (Seq :type "LevelSequenceActor Object Reference"))
  (for _array_element (`self.EventWidgetMapping`)
    (bind _returnvalue (`|GetDataTableRow` _array_element (`local.InName`))
      (:`then`
        (return (`.Widget_10_D05F76FC47EBEDEC836A18B2123F30B4` (break `/Game/Common/Event/FEventWidget` _returnvalue))))))
  (return null))

(fn `GetCrtEventCmd`
  (returns (EventCmd :type "/Game/Common/Event/EventCmds/BPEC_Base Object Reference"))
  (return (`|GetArrayItem` (`self.EventCmds`) (`self.CrtIndex`))))

(fn `GetEventCmdIndexByLabel`
  (params (InLabel :type Name))
  (returns (OutIndex :type Integer))
  (locals (Label :type Name))
  (for (_array_element _array_index) (`self.EventCmds`)
    (if (== (`/Game/Common/Event/EventCmds/BPEC_Base.Label` _array_element) (`local.InLabel`))
      (return _array_index)))
  (return -1))

(fn `GetFlagByName`
  (params (InFlag :type Name))
  (returns (OutBool :type Boolean))
  (locals (Flag :type Integer))
  (return (`BlueprintSetLibrary.Set_Contains` (`self.FlagSet`) (`local.InFlag`))))

(fn `GetSequencePlayer`
  (returns (SequencePlayer :type "LevelSequencePlayer Object Reference"))
  (locals (Name :type String) (Seq :type "LevelSequenceActor Object Reference"))
  (bind _sequenceactor (`self.SequenceActor`))
  (return (select `bool` (`KismetSystemLibrary.IsValid` _sequenceactor) :`true` (`LevelSequenceActor.SequencePlayer` _sequenceactor))))

(fn `PauseSequence`
  (params (InPauseFlag :type Boolean))
  (locals (PauseFlag :type Boolean))
  (bind _sequenceplayer (`LevelSequenceActor.SequencePlayer` (`self.SequenceActor`)))
  (`/Engine/EditorBlueprintResources/StandardMacros.IsValid` (`self.SequenceActor`)
    (:`Is Valid`
      (if (`local.InPauseFlag`)
        (`MovieSceneSequencePlayer.Pause` _sequenceplayer)
        (else
          (`MovieSceneSequencePlayer.Play` _sequenceplayer))))))

(fn `PlaySequence`
  (params (InName :type Name))
  (locals (Name :type String) (Seq :type "LevelSequenceActor Object Reference"))
  (`self.StopSequence`)
  (for _array_element (`self.EventSequenceMapping`)
    (bind _returnvalue (`|GetDataTableRow` _array_element (`local.InName`))
      (:`then`
        (bind _outactor (`LevelSequencePlayer.CreateLevelSequencePlayer` (`.Sequence_7_D05F76FC47EBEDEC836A18B2123F30B4` (break `/Game/Common/Event/FEventSequence` _returnvalue))))
        (set `self.SequenceActor` _outactor)
        (`MovieSceneSequencePlayer.Play` (`LevelSequenceActor.SequencePlayer` (`self.SequenceActor`)))
        (return))))
  (`KismetSystemLibrary.PrintString` (`KismetStringLibrary.Concat_StrStr` "EventCmdComponent::PlaySequence not found sequence : " (`KismetStringLibrary.Conv_NameToString` (`local.InName`))) true true (struct :`R` 1.0 :`B` 1.0 :`A` 1.0)))

(fn `PlaySound2D`
  (params (InName :type "Object Object Reference"))
  (locals (Name :type String))
  (`self.StopSound2D` (`local.InName`))
  (for _array_element (`self.EventSoundMapping`)
    (bind _returnvalue (`|GetDataTableRow` _array_element (`local.InName`))
      (:`then`
        (bind _returnvalue_2 (`GameplayStatics.SpawnSound2D` (`.Sound_4_D05F76FC47EBEDEC836A18B2123F30B4` (break `/Game/Common/Event/FEventSound` _returnvalue)) 1.0 1.0 0.0 null))
        (`BlueprintMapLibrary.Map_Add` (`self.PlayingSoundMapping`) (`local.InName`) _returnvalue_2)))))

(fn `RemoveEventCmdClassMapping`
  (params (InDataTable :type "CompositeDataTable Object Reference"))
  (`KismetArrayLibrary.Array_RemoveItem` (`self.EventCmdClassMapping`) InDataTable))

(fn `RemoveEventMontageMapping`
  (params (InDataTable :type "CompositeDataTable Object Reference"))
  (`KismetArrayLibrary.Array_RemoveItem` (`self.EventMontageMapping`) InDataTable))

(fn `RemoveEventSequenceMapping`
  (params (InDataTable :type "CompositeDataTable Object Reference"))
  (`KismetArrayLibrary.Array_RemoveItem` (`self.EventSequenceMapping`) InDataTable))

(fn `RemoveEventSoundMapping`
  (params (InDataTable :type "CompositeDataTable Object Reference"))
  (`KismetArrayLibrary.Array_RemoveItem` (`self.EventSoundMapping`) InDataTable))

(fn `RemoveEventWidgetMapping`
  (params (InDataTable :type "CompositeDataTable Object Reference"))
  (`KismetArrayLibrary.Array_RemoveItem` (`self.EventWidgetMapping`) InDataTable))

(fn `SetFlagByName`
  (params (InFlag :type Name) (InBool :type Boolean))
  (locals (ParamFlag :type String) (ParamBool :type Boolean) (Flag :type Integer))
  (if InBool
    (`BlueprintSetLibrary.Set_Add` (`self.FlagSet`) (`local.InFlag`))
    (else
      (`BlueprintSetLibrary.Set_Remove` (`self.FlagSet`) (`local.InFlag`)))))

(fn `Start`
  (params (InLabel :type Name))
  (returns (OutResult :type "/Game/Common/Event/EEventCmdResult Enum"))
  (locals (ParamEventCommands :type "Array of /Game/Common/Event/EventCmds/BPEC_Base Object Reference") (Label :type Name) (DataTable :type "DataTable Object Reference"))
  (`/Engine/EditorBlueprintResources/StandardMacros.IsValid` (`self.EventDataTable`)
    (:`Is Valid`
      (if (>= (`self.CrtIndex`) 0)
        (return "NewEnumerator2")
        (else
          (`self.CreateEventCmds` (`self.EventDataTable`))
          (set `self.CrtIndex` (`self.GetEventCmdIndexByLabel` (`local.InLabel`)))
          (if (>= (`self.CrtIndex`) 0)
            (`self.Exec`)
            (return "NewEnumerator0")
            (else
              (return "NewEnumerator3"))))))
    (:`Is Not Valid`
      (return "NewEnumerator4"))))

(fn `StopSequence`
  (`/Engine/EditorBlueprintResources/StandardMacros.IsValid` (`self.SequenceActor`)
    (:`Is Valid`
      (`MovieSceneSequencePlayer.Stop` (`LevelSequenceActor.SequencePlayer` (`self.SequenceActor`)))
      (`Actor.K2_DestroyActor` (`self.SequenceActor`)))))

(fn `StopSound2D`
  (params (InName :type Name) (InDuration :type "Float (double-precision)"))
  (locals (Name :type String) (Duration :type "Float (double-precision)") (Elem :type "AudioComponent Object Reference"))
  (bind (_value _returnvalue) (`BlueprintMapLibrary.Map_Find` (`self.PlayingSoundMapping`) (`local.InName`)))
  (if (== (`local.InName`) "None")
    (bind _keys (`BlueprintMapLibrary.Map_Keys` (`self.PlayingSoundMapping`)))
    (for _array_element _keys
      (`AudioComponent.FadeOut` (`BlueprintMapLibrary.Map_Find` (`self.PlayingSoundMapping`) _array_element) (`local.InDuration`) 0.0 "Linear"))
    (`BlueprintMapLibrary.Map_Clear` (`self.PlayingSoundMapping`))
    (elif _returnvalue
      (`AudioComponent.FadeOut` _value (`local.InDuration`) 0.0 "Linear")
      (`BlueprintMapLibrary.Map_Remove` (`self.PlayingSoundMapping`) (`local.InName`)))))